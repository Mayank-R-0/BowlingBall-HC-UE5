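; BP_Pins is a bowling-pin obstacle actor that removes itself after the ball hits it.
; When a BP_FollowBall overlaps it, it waits two seconds and then destroys itself.
; Getter functions report its obstacle type, pin count and number, plus a fixed end-level type.
; Collision-disable, debug print and impulse nodes remain in the graph but are unconnected and never run.
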(event `self.ReceiveBeginPlay`)

(event `self.ReceiveActorBeginOverlap`
  (params (OtherActor :type "Actor Object Reference"))
  (cast `/Game/BP_FollowBall` OtherActor)
  (`KismetSystemLibrary.Delay` 2.0)
  (`self.K2_DestroyActor`))

(fn `GetEndLevelType`
  (returns (EndLevelType :type "/Game/Blueprints/Enumerations/EndLevelType Enum"))
  (return "NewEnumerator4"))

(fn `GetObstType`
  (returns (Type :type "/Game/ObstacleType Enum"))
  (return (`self.ObstacleType`)))

(fn `GetPinsCount`
  (returns (Count :type "/Game/Obstacles/Pins/PinsCount Enum") (Number :type Integer))
  (return (`self.PinsCount`) (`self.Number`)))

(fn `UserConstructionScript`)