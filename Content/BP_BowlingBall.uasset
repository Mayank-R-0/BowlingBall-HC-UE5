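; Player bowling ball that leads a five-column swarm of follower balls along a spline track, steered by swipes.
; Touch drags shift BP_FollowSpline's offset; each tick the ball lerps to its reference point, updates the camera and advances chained BP_FollowBalls.
; TypeInterface overlaps add or remove balls, boost speed, collect gems, enable physics or trigger one of three endings.
; The third ending launches followers by impulse while touching, relinking each column's chain.
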(event `self.ReceiveTick`
  (params (DeltaSeconds :type "Float (single-precision)"))
  (bind (_returnvalue_location _returnvalue_rotation) (`KismetMathLibrary.BreakTransform` (`SceneComponent.K2_GetComponentToWorld` (`/Game/Controls/BP_FollowSpline.CameraReferencePoint` (`self.SplineRefr`)))))
  ;[1 1 1] Event Tick
  (if (`self.GameStarted`)
    (`|ExecutionSequence`
      (:`then_0`
        ;;[0 1 0] Calculating rotation and location offset from screen touch
        (if (not (`self.StopHorizontalMovement`))
          (`/Engine/EditorBlueprintResources/StandardMacros.Gate` true :!label _label
            (:`Exit`
              (bind _returnvalue_x (`KismetMathLibrary.BreakVector` (- (stale `InputTouch` Location) (`self.TouchStartLocation`))))
              (bind _output_get (set `self.MouseAxisValue` _returnvalue_x))
              (set `/Game/Controls/BP_FollowSpline.Offset` (`KismetMathLibrary.FClamp` (+ (`/Game/Controls/BP_FollowSpline.Offset` (`self.SplineRefr`)) (* _output_get (`self.SwipeSensitivity`))) -400.0 400.0) (`self.SplineRefr`))
              (set `self.TouchStartLocation` (stale `InputTouch` Location))))))
      (:`then_1`
        ;;[0 1 0] Moving Main ball
        (`self.Move`)
        (if (not (`self.StopCamera`))
          (`self.K2_SetActorLocationAndRotation` (`self.FollowCamera`) _returnvalue_location _returnvalue_rotation false false)))
      (:`then_2`
        ;;[0 1 0] Updating following balls location
        (`self.UpdateFollowBallLastLocation`)))))

(event `InputTouch`
  (params (Location :type "Vector Structure") (FingerIndex :type "ETouchIndex Enum"))
  ;[1 1 1] Event Tick
  ;;[0 1 0] Calculating rotation and location offset from screen touch
  (:`Pressed`
    (set `self.TouchStartLocation` Location)
    (`self.HandleTouchPressed`))
  (:`Released`
    (set `self.TouchPressed` false)
    (set `self.MouseAxisValue` 0.0)
    (goto _label :!via `Close`))
  (:`Moved`
    (set `self.TouchPressed` true)
    (goto _label :!via `Open`)))

(event `self.ReceiveBeginPlay`
  ;[1 1 1] Begin Play
  (`self.SpawnBallsBackwards` 50)
  (`KismetSystemLibrary.ExecuteConsoleCommand` "t.MaxFPS 60" null)
  (set `PlayerController.bShowMouseCursor` true (`GameplayStatics.GetPlayerController` 0))
  (bind _asbp_game_instance (cast `/Game/Blueprints/CoreClasses/BP_GameInstance` (`GameplayStatics.GetGameInstance`)))
  (bind _output_get (set `self.BP_Game_Instance` _asbp_game_instance))
  (set `/Game/Blueprints/CoreClasses/BP_GameInstance.CurrentLevelGems` (`self.Gem Count`) _output_get)
  (bind _returnvalue (`GameplayStatics.GetActorOfClass` "/Game/Controls/BP_FollowSpline.BP_FollowSpline_C"))
  (bind _output_get_2 (set `self.SplineRefr` _returnvalue))
  (set `/Game/Controls/BP_FollowSpline.MovementSpeed` (`self.MovementSpeed`) _output_get_2)
  (bind _returnvalue_2 (`GameplayStatics.GetActorOfClass` "/Game/Controls/BP_FollowCamera.BP_FollowCamera_C"))
  (bind _output_get_3 (set `self.FollowCamera` _returnvalue_2))
  (`PlayerController.SetViewTargetWithBlend` (`GameplayStatics.GetPlayerController` 0) _output_get_3 0.0 "VTBlend_Linear" 0.0 false)
  (bind _returnvalue_3 (`|CreateWidget` "/Game/UI/MainMenu.MainMenu_C" (`GameplayStatics.GetPlayerController` 0)))
  (bind _output_get_4 (set `self.MainUI` _returnvalue_3))
  (`UserWidget.AddToPlayerScreen` _output_get_4 0)
  (`GameplayStatics.SetGamePaused` true))

(event `TotalBallsCount`
  ;[1 1 1] Calculating total count of balls currently
  (set `self.Total Length` (+ (`KismetArrayLibrary.Array_Length` (`self.ColumnOne`)) (`KismetArrayLibrary.Array_Length` (`self.ColumnOne`)) (`KismetArrayLibrary.Array_Length` (`self.ColumnOne`)) (`KismetArrayLibrary.Array_Length` (`self.ColumnOne`)) (`KismetArrayLibrary.Array_Length` (`self.ColumnOne`)))))

(event `Move`
  (bind (_returnvalue_x _returnvalue_y _returnvalue_z) (`KismetMathLibrary.BreakVector` (`self.K2_GetActorLocation`)))
  (bind _returnvalue (`SceneComponent.K2_GetComponentToWorld` (`/Game/Controls/BP_FollowSpline.ReferencePoint` (`self.SplineRefr`))))
  (bind _returnvalue_2 (`KismetMathLibrary.SelectFloat` (.z (.location _returnvalue)) _returnvalue_z (`self.StopForwardMovement`)))
  ;[1 1 1] Forward Movement and Rotation applied
  (set `self.Offset ` (`KismetMathLibrary.FClamp` (`KismetMathLibrary.FInterpTo` (`self.Offset `) (`self.MouseAxisValue`) (`GameplayStatics.GetWorldDeltaSeconds`) (`self.RotationSpeed`)) -50.0 50.0))
  (`self.K2_SetActorTransform` (`KismetMathLibrary.MakeTransform` (`KismetMathLibrary.VLerp` (`KismetMathLibrary.MakeVector` _returnvalue_x _returnvalue_y _returnvalue_2) (`KismetMathLibrary.MakeVector` (.x (.location _returnvalue)) (.y (.location _returnvalue)) _returnvalue_2) (* (`GameplayStatics.GetWorldDeltaSeconds`) (`self.SwipeSpeed`))) (`KismetMathLibrary.SelectRotator` (struct) (`KismetMathLibrary.MakeRotator` (.roll (.rotation _returnvalue)) (.pitch (.rotation _returnvalue)) (+ (.yaw (.rotation _returnvalue)) (`self.Offset `))) (`self.End Level Three Triggered`)) (`self.GetActorScale3D`))))

(event `self.BoxCollider.OnComponentBeginOverlap`
  (params (OverlappedComponent :type "PrimitiveComponent Object Reference") (OtherActor :type "Actor Object Reference") (OtherComp :type "PrimitiveComponent Object Reference") (OtherBodyIndex :type Integer) (bFromSweep :type Boolean) (SweepResult :type "HitResult Structure (by ref)"))
  (bind _bp_game_instance (`self.BP_Game_Instance`))
  (bind _charactermovement (`self.CharacterMovement`))
  ;[1 0.9931 0.8873] Ball Collision Detection with various obstacles and End Level Handles
  (bind _astype_interface (cast `/Game/TypeInterface` OtherActor))
  (bind _type (`/Game/TypeInterface.GetObstType` _astype_interface))
  (switch `/Game/ObstacleType` _type
    (:`NewEnumerator0`)
    (:`NewEnumerator1`)
    (:`NewEnumerator2`)
    (:`NewEnumerator3`
      ;;[1 0 0.0111] Bowling Pin Collision
      (`self.SetActorHiddenInGame` OtherActor false)
      (`self.RemoveFromBowlingPin` 5))
    (:`NewEnumerator4`
      ;;[0.1451 0 1] Escalator Collision
      (bind _output_get (set `self.MovementSpeed` (+ (`self.MovementSpeed`) 200.0)))
      (set `/Game/Controls/BP_FollowSpline.MovementSpeed` _output_get (`self.SplineRefr`))
      (`KismetSystemLibrary.Delay` 2.0)
      (bind _output_get_2 (set `self.MovementSpeed` (+ (`self.MovementSpeed`) -200.0)))
      (set `/Game/Controls/BP_FollowSpline.MovementSpeed` _output_get_2 (`self.SplineRefr`)))
    (:`NewEnumerator6`
      ;;[1 0.7841 0] Bowling Balls Collision
      (`self.SpawnBallsBackwards` 5)
      (`self.K2_DestroyActor` OtherActor))
    (:`NewEnumerator7`
      ;;[0 0.8505 1] Gems Collision
      (bind _result (`/Engine/EditorBlueprintResources/StandardMacros.IncrementInt` (`self.Gem Count`))
        (:`  `
          (set `/Game/Blueprints/CoreClasses/BP_GameInstance.CurrentLevelGems` _result _bp_game_instance)
          (`/Game/Blueprints/CoreClasses/BP_GameInstance.UpdateTotalGems` _bp_game_instance 1)
          (`self.K2_DestroyActor` OtherActor))))
    (:`NewEnumerator9`
      ;;[1 0.9522 0] End Levels Handling
      (`/Engine/EditorBlueprintResources/StandardMacros.DoOnce` false
        (:`Completed`
          (bind _endleveltype (`/Game/TypeInterface.GetEndLevelType` _astype_interface))
          (switch `/Game/Blueprints/Enumerations/EndLevelType` _endleveltype
            (:`NewEnumerator0`
              ;;;[0 1 1] End Level One
              (set `self.StopForwardMovement` true)
              (set `self.StopHorizontalMovement` true)
              (set `CharacterMovementComponent.GravityScale` 0.0 _charactermovement)
              (set `CharacterMovementComponent.bApplyGravityWhileJumping` false _charactermovement)
              (set `self.StopCamera` true)
              (`self.AttachAllBallsToMainBall`)
              (`/Game/Controls/BP_FollowCamera.LerpCamera` (`self.FollowCamera`) 1000.0)
              (set `/Game/Controls/BP_FollowSpline.Offset` 0.0 (`self.SplineRefr`))
              (`KismetSystemLibrary.Delay` (`self.EndTime`))
              (`/Game/UI/MainMenu.ShowLevelFinish` (`self.MainUI`)))
            (:`NewEnumerator1`
              ;;;[0 1 1] End Level Two
              (`/Engine/EditorBlueprintResources/StandardMacros.DoOnce` false
                (:`Completed`
                  (bind _output_get_3 (set `self.MovementSpeed` (+ (`self.MovementSpeed`) -500.0)))
                  (set `/Game/Controls/BP_FollowSpline.MovementSpeed` _output_get_3 (`self.SplineRefr`))
                  (`KismetSystemLibrary.Delay` (`self.EndTime`))
                  (`/Game/UI/MainMenu.ShowLevelFinish` (`self.MainUI`)))))
            (:`NewEnumerator2`
              ;;;[0 1 1] End Level Three
              (set `self.StopForwardMovement` true)
              (`self.TotalBallsCount`)
              (set `self.StopCamera` true)
              (set `self.End Level Three Triggered` true)
              (`self.AttachAllBallsToMainBall`)
              (`KismetSystemLibrary.K2_SetTimerDelegate` (delegate `StartendLevelThree`) 0.01 true))))))
    (:`NewEnumerator10`
      ;;[0 0 1] Simulate Physics to All balls
      (`self.SimulatePhysicsOnFollowBalls`))))

(event `StartendLevelThree`
  ;[1 0.9931 0.8873] Ball Collision Detection with various obstacles and End Level Handles
  ;;[1 0.9522 0] End Levels Handling
  ;;;[0 1 1] End Level Three
  (bind _output_get (set `self.TimeElapsed` (+ (`self.TimeElapsed`) (`GameplayStatics.GetWorldDeltaSeconds`))))
  (if (and (>= _output_get 0.5) (`self.TouchPressed`))
    (`self.Throw Ball` (`self.CurrentBallCount`))
    (set `self.TimeElapsed` 0.0)))

(fn `AttachAllBallsToMainBall`
  (for _array_element (`self.ColumnOne`)
    (`self.K2_AttachToActor` _array_element self "None" "KeepWorld" "KeepWorld" "KeepWorld" true))
  (for _array_element_2 (`self.ColumnTwo`)
    (`self.K2_AttachToActor` _array_element_2 self "None" "KeepWorld" "KeepWorld" "KeepWorld" true))
  (for _array_element_3 (`self.ColumnThree`)
    (`self.K2_AttachToActor` _array_element_3 self "None" "KeepWorld" "KeepWorld" "KeepWorld" true))
  (for _array_element_4 (`self.ColumnFour`)
    (`self.K2_AttachToActor` _array_element_4 self "None" "KeepWorld" "KeepWorld" "KeepWorld" true))
  (for _array_element_5 (`self.ColumnFive`)
    (`self.K2_AttachToActor` _array_element_5 self "None" "KeepWorld" "KeepWorld" "KeepWorld" true)))

(fn `FollowBallDestroyed`
  (params (ColumnNumber :type Integer) (Index :type Integer) (Head :type "Actor Object Reference") (Xoff :type "Float (double-precision)") (YOff :type "Float (double-precision)"))
  (switch `int` ColumnNumber
    (:`0`
      (`/Game/BP_FollowBall.Update Head` (`|GetArrayItem` (`self.ColumnOne`) (+ Index 1)) Head Xoff YOff Index)
      (`KismetArrayLibrary.Array_Remove` (`self.ColumnOne`) Index))
    (:`1`
      (`/Game/BP_FollowBall.Update Head` (`|GetArrayItem` (`self.ColumnTwo`) (+ Index 1)) Head Xoff YOff Index)
      (`KismetArrayLibrary.Array_Remove` (`self.ColumnTwo`) Index))
    (:`2`
      (`/Game/BP_FollowBall.Update Head` (`|GetArrayItem` (`self.ColumnThree`) (+ Index 1)) Head Xoff YOff Index)
      (`KismetArrayLibrary.Array_Remove` (`self.ColumnThree`) Index))
    (:`3`
      (`/Game/BP_FollowBall.Update Head` (`|GetArrayItem` (`self.ColumnFour`) (+ Index 1)) Head Xoff YOff Index)
      (`KismetArrayLibrary.Array_Remove` (`self.ColumnFour`) Index))
    (:`4`
      (`/Game/BP_FollowBall.Update Head` (`|GetArrayItem` (`self.ColumnFive`) (+ Index 1)) Head Xoff YOff Index)
      (`KismetArrayLibrary.Array_Remove` (`self.ColumnFive`) Index))))

(fn `HandleTouchPressed`
  ;[1 1 1] Throw Ball once for End Level Three
  (`self.Throw Ball` (`self.CurrentBallCount`)))

(fn `RemoveFromBowlingPin`
  (params (Count :type Integer))
  (bind _columnone (`self.ColumnOne`))
  (bind _columntwo (`self.ColumnTwo`))
  (bind _columnthree (`self.ColumnThree`))
  (bind _columnfour (`self.ColumnFour`))
  (bind _columnfive (`self.ColumnFive`))
  (bind _output (`|GetArrayItem` _columnfive (`KismetArrayLibrary.Array_LastIndex` _columnfive)))
  (bind _output_2 (`|GetArrayItem` _columnone (`KismetArrayLibrary.Array_LastIndex` _columnone)))
  (bind _output_3 (`|GetArrayItem` _columntwo (`KismetArrayLibrary.Array_LastIndex` _columntwo)))
  (bind _output_4 (`|GetArrayItem` _columnthree (`KismetArrayLibrary.Array_LastIndex` _columnthree)))
  (bind _output_5 (`|GetArrayItem` _columnfour (`KismetArrayLibrary.Array_LastIndex` _columnfour)))
  (for _index (range Count)
    (switch `int` (mod _index 5)
      (:`0`
        (`self.K2_DestroyActor` _output_2)
        (`KismetArrayLibrary.Array_RemoveItem` _columnone _output_2))
      (:`1`
        (`self.K2_DestroyActor` _output_3)
        (`KismetArrayLibrary.Array_RemoveItem` _columntwo _output_3))
      (:`2`
        (`self.K2_DestroyActor` _output_4)
        (`KismetArrayLibrary.Array_RemoveItem` _columnthree _output_4))
      (:`3`
        (`self.K2_DestroyActor` _output_5)
        (`KismetArrayLibrary.Array_RemoveItem` _columnfour _output_5))
      (:`4`
        (`self.K2_DestroyActor` _output)
        (`KismetArrayLibrary.Array_RemoveItem` _columnfive _output)))))

(fn `ResetOffsetOfBalls`
  (for _array_element (`self.ColumnOne`)
    (set `/Game/BP_FollowBall.Offset` -50.0 _array_element)))

(fn `SimulatePhysicsOnFollowBalls`
  (for _array_element (`self.ColumnOne`)
    (`self.SimulatePhysicsSettings` (`/Game/BP_FollowBall.Sphere` _array_element)))
  (for _array_element_2 (`self.ColumnTwo`)
    (`self.SimulatePhysicsSettings` (`/Game/BP_FollowBall.Sphere` _array_element_2)))
  (for _array_element_3 (`self.ColumnThree`)
    (`self.SimulatePhysicsSettings` (`/Game/BP_FollowBall.Sphere` _array_element_3)))
  (for _array_element_4 (`self.ColumnFour`)
    (`self.SimulatePhysicsSettings` (`/Game/BP_FollowBall.Sphere` _array_element_4)))
  (for _array_element_5 (`self.ColumnFive`)
    (`self.SimulatePhysicsSettings` (`/Game/BP_FollowBall.Sphere` _array_element_5))))

(fn `SimulatePhysicsSettings`
  (params (PrimitiveComponent :type "PrimitiveComponent Object Reference"))
  (`PrimitiveComponent.SetSimulatePhysics` PrimitiveComponent true)
  (`PrimitiveComponent.SetCollisionEnabled` PrimitiveComponent "QueryAndPhysics")
  (`PrimitiveComponent.SetCollisionResponseToChannel` PrimitiveComponent "ECC_WorldStatic" "ECR_Block"))

(fn `SpawnBallsBackwards`
  (params (NumberOfBalls :type Integer))
  (locals (SpawnLocation :type "Vector Structure" :default (0.0 0.0 0.0)))
  (bind _columntwo (`self.ColumnTwo`))
  (bind _columnthree (`self.ColumnThree`))
  (bind _columnfour (`self.ColumnFour`))
  (bind _columnfive (`self.ColumnFive`))
  (bind _columnone (`self.ColumnOne`))
  (bind (_returnvalue_x _returnvalue_y) (`KismetMathLibrary.BreakVector` (`SceneComponent.K2_GetComponentLocation` (`/Game/Controls/BP_FollowCamera.Camera` (`self.FollowCamera`)))))
  (bind _output (`|GetArrayItem` _columnone (`KismetArrayLibrary.Array_LastIndex` _columnone)))
  (bind _output_2 (`|GetArrayItem` _columnfive (`KismetArrayLibrary.Array_LastIndex` _columnfive)))
  (bind _output_3 (`|GetArrayItem` _columntwo (`KismetArrayLibrary.Array_LastIndex` _columntwo)))
  (bind _output_4 (`|GetArrayItem` _columnthree (`KismetArrayLibrary.Array_LastIndex` _columnthree)))
  (bind _output_5 (`|GetArrayItem` _columnfour (`KismetArrayLibrary.Array_LastIndex` _columnfour)))
  (bind _returnvalue (`KismetSystemLibrary.IsValid` _output_2))
  (bind _returnvalue_2 (`KismetSystemLibrary.IsValid` _output_3))
  (bind _returnvalue_3 (`KismetSystemLibrary.IsValid` _output))
  (bind _returnvalue_4 (`KismetSystemLibrary.IsValid` _output_4))
  (bind _returnvalue_5 (`KismetSystemLibrary.IsValid` _output_5))
  (set `local.SpawnLocation` (`KismetMathLibrary.MakeVector` _returnvalue_x _returnvalue_y))
  (for _index (range NumberOfBalls)
    (switch `int` (mod _index 5)
      (:`0`
        (bind _returnvalue_6 (`|SpawnActorFromClass` "/Game/BP_FollowBall.BP_FollowBall_C" (`KismetMathLibrary.MakeTransform` (`local.SpawnLocation`)) "Undefined" "OverrideRootScale" null (select `bool` _returnvalue_3 :`false` self :`true` _output :!type "Actor Object Reference") -10.0 (`KismetMathLibrary.SelectFloat` 0.0 -100.0 _returnvalue_3) self null))
        (bind _returnvalue_7 (`KismetArrayLibrary.Array_Add` (`self.ColumnOne`) _returnvalue_6))
        (set `/Game/BP_FollowBall.Index` _returnvalue_7 _returnvalue_6)
        (set `/Game/BP_FollowBall.ColumnNumber` 0 _returnvalue_6)
        (`PrimitiveComponent.SetMaterial` (`/Game/BP_FollowBall.Sphere` _returnvalue_6) 0 "/Game/Materials/BallColumns/ColOne.ColOne"))
      (:`1`
        (bind _returnvalue_8 (`|SpawnActorFromClass` "/Game/BP_FollowBall.BP_FollowBall_C" (`KismetMathLibrary.MakeTransform` (`local.SpawnLocation`)) "Undefined" "OverrideRootScale" null (select `bool` _returnvalue_2 :`false` self :`true` _output_3 :!type "Actor Object Reference") -10.0 (`KismetMathLibrary.SelectFloat` 0.0 -50.0 _returnvalue_2) self null))
        (bind _returnvalue_9 (`KismetArrayLibrary.Array_Add` (`self.ColumnTwo`) _returnvalue_8))
        (set `/Game/BP_FollowBall.Index` _returnvalue_9 _returnvalue_8)
        (set `/Game/BP_FollowBall.ColumnNumber` 1 _returnvalue_8)
        (`PrimitiveComponent.SetMaterial` (`/Game/BP_FollowBall.Sphere` _returnvalue_8) 0 "/Game/Materials/BallColumns/ColTwo.ColTwo"))
      (:`2`
        (bind _returnvalue_10 (`|SpawnActorFromClass` "/Game/BP_FollowBall.BP_FollowBall_C" (`KismetMathLibrary.MakeTransform` (`local.SpawnLocation`)) "Undefined" "OverrideRootScale" null (select `bool` _returnvalue_4 :`false` self :`true` _output_4 :!type "Actor Object Reference") -10.0 (`KismetMathLibrary.SelectFloat` 0.0 0.0 _returnvalue_4) self null))
        (bind _returnvalue_11 (`KismetArrayLibrary.Array_Add` (`self.ColumnThree`) _returnvalue_10))
        (set `/Game/BP_FollowBall.Index` _returnvalue_11 _returnvalue_10)
        (set `/Game/BP_FollowBall.ColumnNumber` 2 _returnvalue_10)
        (`PrimitiveComponent.SetMaterial` (`/Game/BP_FollowBall.Sphere` _returnvalue_10) 0 "/Game/Materials/BallColumns/ColThree.ColThree"))
      (:`3`
        (bind _returnvalue_12 (`|SpawnActorFromClass` "/Game/BP_FollowBall.BP_FollowBall_C" (`KismetMathLibrary.MakeTransform` (`local.SpawnLocation`)) "Undefined" "OverrideRootScale" null (select `bool` _returnvalue_5 :`false` self :`true` _output_5 :!type "Actor Object Reference") -10.0 (`KismetMathLibrary.SelectFloat` 0.0 50.0 _returnvalue_5) self null))
        (bind _returnvalue_13 (`KismetArrayLibrary.Array_Add` (`self.ColumnFour`) _returnvalue_12))
        (set `/Game/BP_FollowBall.Index` _returnvalue_13 _returnvalue_12)
        (set `/Game/BP_FollowBall.ColumnNumber` 3 _returnvalue_12)
        (`PrimitiveComponent.SetMaterial` (`/Game/BP_FollowBall.Sphere` _returnvalue_12) 0 "/Game/Materials/BallColumns/ColFour.ColFour"))
      (:`4`
        (bind _returnvalue_14 (`|SpawnActorFromClass` "/Game/BP_FollowBall.BP_FollowBall_C" (`KismetMathLibrary.MakeTransform` (`local.SpawnLocation`)) "Undefined" "OverrideRootScale" null (select `bool` _returnvalue :`false` self :`true` _output_2 :!type "Actor Object Reference") -10.0 (`KismetMathLibrary.SelectFloat` 0.0 100.0 _returnvalue) self null))
        (bind _returnvalue_15 (`KismetArrayLibrary.Array_Add` (`self.ColumnFive`) _returnvalue_14))
        (set `/Game/BP_FollowBall.Index` _returnvalue_15 _returnvalue_14)
        (set `/Game/BP_FollowBall.ColumnNumber` 4 _returnvalue_14)
        (`PrimitiveComponent.SetMaterial` (`/Game/BP_FollowBall.Sphere` _returnvalue_14) 0 "/Game/Materials/BallColumns/ColFive.ColFive")))))

(fn `Throw Ball`
  (params (Index :type Integer))
  (locals (CurentBall :type "/Game/BP_FollowBall Object Reference"))
  (bind _columnthree (`self.ColumnThree`))
  (bind _columntwo (`self.ColumnTwo`))
  (bind _columnone (`self.ColumnOne`))
  (bind _columnfour (`self.ColumnFour`))
  (bind _columnfive (`self.ColumnFive`))
  (bind _output (`|GetArrayItem` _columnone))
  (bind _output_2 (`|GetArrayItem` _columnfour))
  (bind _output_3 (`|GetArrayItem` _columnthree))
  (bind _output_4 (`|GetArrayItem` _columntwo))
  (bind _output_5 (`|GetArrayItem` _columnfive))
  (bind _sphere (`/Game/BP_FollowBall.Sphere` _output_3))
  (bind _sphere_2 (`/Game/BP_FollowBall.Sphere` _output_4))
  (bind _sphere_3 (`/Game/BP_FollowBall.Sphere` _output))
  (bind _sphere_4 (`/Game/BP_FollowBall.Sphere` _output_5))
  (bind _sphere_5 (`/Game/BP_FollowBall.Sphere` _output_2))
  (if (and (`self.End Level Three Triggered`) (< (`self.CurrentBallCount`) (`self.Total Length`)))
    (`/Engine/EditorBlueprintResources/StandardMacros.IncrementInt` (`self.CurrentBallCount`)
      (:`  `
        (switch `int` (mod Index 5)
          (:`0`
            (`self.UpdateHeadOfBall` _output (`|GetArrayItem` _columnone 1))
            (`self.SimulatePhysicsSettings` _sphere_3)
            (`PrimitiveComponent.AddImpulse` _sphere_3 (1000.0 0.0 0.0) "None" true)
            (`KismetArrayLibrary.Array_Remove` (`self.ColumnOne`)))
          (:`1`
            (`self.UpdateHeadOfBall` _output_4 (`|GetArrayItem` _columntwo 1))
            (`self.SimulatePhysicsSettings` _sphere_2)
            (`PrimitiveComponent.AddImpulse` _sphere_2 (1000.0 0.0 0.0) "None" true)
            (`KismetArrayLibrary.Array_Remove` (`self.ColumnTwo`)))
          (:`2`
            (`self.UpdateHeadOfBall` _output_3 (`|GetArrayItem` _columnthree 1))
            (`self.SimulatePhysicsSettings` _sphere)
            (`PrimitiveComponent.AddImpulse` _sphere (1000.0 0.0 0.0) "None" true)
            (`KismetArrayLibrary.Array_Remove` (`self.ColumnThree`)))
          (:`3`
            (`self.UpdateHeadOfBall` _output_2 (`|GetArrayItem` _columnfour 1))
            (`self.SimulatePhysicsSettings` _sphere_5)
            (`PrimitiveComponent.AddImpulse` _sphere_5 (1000.0 0.0 0.0) "None" true)
            (`KismetArrayLibrary.Array_Remove` (`self.ColumnFour`)))
          (:`4`
            (`self.UpdateHeadOfBall` _output_5 (`|GetArrayItem` _columnfive 1))
            (`self.SimulatePhysicsSettings` _sphere_4)
            (`PrimitiveComponent.AddImpulse` _sphere_4 (1000.0 0.0 0.0) "None" true)
            (`KismetArrayLibrary.Array_Remove` (`self.ColumnFive`))))))))

(fn `UpdateFollowBallLastLocation`
  (locals (ColOne :type "Array of /Game/BP_FollowBall Object Reference") (ColTwo :type "Array of /Game/BP_FollowBall Object Reference") (ColThree :type "Array of /Game/BP_FollowBall Object Reference") (ColFour :type "Array of /Game/BP_FollowBall Object Reference") (ColFive :type "Array of /Game/BP_FollowBall Object Reference"))
  (if (not (`self.StopForwardMovement`))
    (set `local.ColOne` (`self.ColumnOne`))
    (set `local.ColTwo` (`self.ColumnTwo`))
    (set `local.ColThree` (`self.ColumnThree`))
    (set `local.ColFour` (`self.ColumnFour`))
    (set `local.ColFive` (`self.ColumnFive`))
    (for _array_element (`local.ColOne`)
      (`/Engine/EditorBlueprintResources/StandardMacros.IsValid` _array_element
        (:`Is Valid`
          (`/Game/BP_FollowBall.FollowTarget` _array_element))))
    (for _array_element_2 (`local.ColTwo`)
      (`/Engine/EditorBlueprintResources/StandardMacros.IsValid` _array_element_2
        (:`Is Valid`
          (`/Game/BP_FollowBall.FollowTarget` _array_element_2))))
    (for _array_element_3 (`local.ColThree`)
      (`/Engine/EditorBlueprintResources/StandardMacros.IsValid` _array_element_3
        (:`Is Valid`
          (`/Game/BP_FollowBall.FollowTarget` _array_element_3))))
    (for _array_element_4 (`local.ColFour`)
      (`/Engine/EditorBlueprintResources/StandardMacros.IsValid` _array_element_4
        (:`Is Valid`
          (`/Game/BP_FollowBall.FollowTarget` _array_element_4))))
    (for _array_element_5 (`local.ColFive`)
      (`/Engine/EditorBlueprintResources/StandardMacros.IsValid` _array_element_5
        (:`Is Valid`
          (`/Game/BP_FollowBall.FollowTarget` _array_element_5))))))

(fn `UpdateHeadOfBall`
  (params (PreviousBall :type "/Game/BP_FollowBall Object Reference") (NextBall :type "/Game/BP_FollowBall Object Reference"))
  (set `/Game/BP_FollowBall.FollowHead` (`/Game/BP_FollowBall.FollowHead` PreviousBall) NextBall)
  (set `/Game/BP_FollowBall.Index` (`/Game/BP_FollowBall.Index` PreviousBall) NextBall)
  (set `/Game/BP_FollowBall.Offset` (`/Game/BP_FollowBall.Offset` PreviousBall) NextBall)
  (set `/Game/BP_FollowBall.Yoffset` (`/Game/BP_FollowBall.Yoffset` PreviousBall) NextBall))

(fn `UserConstructionScript`)