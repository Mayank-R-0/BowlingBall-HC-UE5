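; End-level actor that awards a multiplier and removes balls from the bowling ball as its numbered ball targets are hit.
; On BeginPlay it gives twelve text renders random numbers within a set range and caches the BP_BowlingBall in the level.
; Each target's first overlap hides it and passes its number and tier, X2 to X10, to RemoveBallsEndLevelFour.
; A separate impulse collider turns on physics for overlapping components and launches them with a random impulse.
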(event `self.Ball1.OnComponentBeginOverlap`
  (params (OverlappedComponent :type "PrimitiveComponent Object Reference") (OtherActor :type "Actor Object Reference") (OtherComp :type "PrimitiveComponent Object Reference") (OtherBodyIndex :type Integer) (bFromSweep :type Boolean) (SweepResult :type "HitResult Structure (by ref)"))
  (`/Engine/EditorBlueprintResources/StandardMacros.DoOnce` false
    (:`Completed`
      (`SceneComponent.SetHiddenInGame` OverlappedComponent true true)
      (`/Game/BP_BowlingBall.RemoveBallsEndLevelFour` (`self.Bowling Ball REF`) (`KismetStringLibrary.Conv_StringToInt` (`KismetTextLibrary.Conv_TextToString` (`TextRenderComponent.Text` (`self.Ball1_Text`)))) "X2"))))

(event `self.Ball2.OnComponentBeginOverlap`
  (params (OverlappedComponent :type "PrimitiveComponent Object Reference") (OtherActor :type "Actor Object Reference") (OtherComp :type "PrimitiveComponent Object Reference") (OtherBodyIndex :type Integer) (bFromSweep :type Boolean) (SweepResult :type "HitResult Structure (by ref)"))
  (`/Engine/EditorBlueprintResources/StandardMacros.DoOnce` false
    (:`Completed`
      (`SceneComponent.SetHiddenInGame` OverlappedComponent true true)
      (`/Game/BP_BowlingBall.RemoveBallsEndLevelFour` (`self.Bowling Ball REF`) (`KismetStringLibrary.Conv_StringToInt` (`KismetTextLibrary.Conv_TextToString` (`TextRenderComponent.Text` (`self.Ball2_Text`)))) "X2"))))

(event `self.Ball3.OnComponentBeginOverlap`
  (params (OverlappedComponent :type "PrimitiveComponent Object Reference") (OtherActor :type "Actor Object Reference") (OtherComp :type "PrimitiveComponent Object Reference") (OtherBodyIndex :type Integer) (bFromSweep :type Boolean) (SweepResult :type "HitResult Structure (by ref)"))
  (`/Engine/EditorBlueprintResources/StandardMacros.DoOnce` false
    (:`Completed`
      (`SceneComponent.SetHiddenInGame` OverlappedComponent true true)
      (`/Game/BP_BowlingBall.RemoveBallsEndLevelFour` (`self.Bowling Ball REF`) (`KismetStringLibrary.Conv_StringToInt` (`KismetTextLibrary.Conv_TextToString` (`TextRenderComponent.Text` (`self.Ball3_Text`)))) "X3"))))

(event `self.Ball4.OnComponentBeginOverlap`
  (params (OverlappedComponent :type "PrimitiveComponent Object Reference") (OtherActor :type "Actor Object Reference") (OtherComp :type "PrimitiveComponent Object Reference") (OtherBodyIndex :type Integer) (bFromSweep :type Boolean) (SweepResult :type "HitResult Structure (by ref)"))
  (`/Engine/EditorBlueprintResources/StandardMacros.DoOnce` false
    (:`Completed`
      (`SceneComponent.SetHiddenInGame` OverlappedComponent true true)
      (`/Game/BP_BowlingBall.RemoveBallsEndLevelFour` (`self.Bowling Ball REF`) (`KismetStringLibrary.Conv_StringToInt` (`KismetTextLibrary.Conv_TextToString` (`TextRenderComponent.Text` (`self.Ball4_Text`)))) "X3"))))

(event `self.Ball5.OnComponentBeginOverlap`
  (params (OverlappedComponent :type "PrimitiveComponent Object Reference") (OtherActor :type "Actor Object Reference") (OtherComp :type "PrimitiveComponent Object Reference") (OtherBodyIndex :type Integer) (bFromSweep :type Boolean) (SweepResult :type "HitResult Structure (by ref)"))
  (`/Engine/EditorBlueprintResources/StandardMacros.DoOnce` false
    (:`Completed`
      (`SceneComponent.SetHiddenInGame` OverlappedComponent true true)
      (`/Game/BP_BowlingBall.RemoveBallsEndLevelFour` (`self.Bowling Ball REF`) (`KismetStringLibrary.Conv_StringToInt` (`KismetTextLibrary.Conv_TextToString` (`TextRenderComponent.Text` (`self.Ball5_Text`)))) "X3"))))

(event `self.Ball6.OnComponentBeginOverlap`
  (params (OverlappedComponent :type "PrimitiveComponent Object Reference") (OtherActor :type "Actor Object Reference") (OtherComp :type "PrimitiveComponent Object Reference") (OtherBodyIndex :type Integer) (bFromSweep :type Boolean) (SweepResult :type "HitResult Structure (by ref)"))
  (`/Engine/EditorBlueprintResources/StandardMacros.DoOnce` false
    (:`Completed`
      (`SceneComponent.SetHiddenInGame` OverlappedComponent true true)
      (`/Game/BP_BowlingBall.RemoveBallsEndLevelFour` (`self.Bowling Ball REF`) (`KismetStringLibrary.Conv_StringToInt` (`KismetTextLibrary.Conv_TextToString` (`TextRenderComponent.Text` (`self.Ball6_Text`)))) "X5"))))

(event `self.Ball7.OnComponentBeginOverlap`
  (params (OverlappedComponent :type "PrimitiveComponent Object Reference") (OtherActor :type "Actor Object Reference") (OtherComp :type "PrimitiveComponent Object Reference") (OtherBodyIndex :type Integer) (bFromSweep :type Boolean) (SweepResult :type "HitResult Structure (by ref)"))
  (`/Engine/EditorBlueprintResources/StandardMacros.DoOnce` false
    (:`Completed`
      (`SceneComponent.SetHiddenInGame` OverlappedComponent true true)
      (`/Game/BP_BowlingBall.RemoveBallsEndLevelFour` (`self.Bowling Ball REF`) (`KismetStringLibrary.Conv_StringToInt` (`KismetTextLibrary.Conv_TextToString` (`TextRenderComponent.Text` (`self.Ball7_Text`)))) "X5"))))

(event `self.Ball8.OnComponentBeginOverlap`
  (params (OverlappedComponent :type "PrimitiveComponent Object Reference") (OtherActor :type "Actor Object Reference") (OtherComp :type "PrimitiveComponent Object Reference") (OtherBodyIndex :type Integer) (bFromSweep :type Boolean) (SweepResult :type "HitResult Structure (by ref)"))
  (`/Engine/EditorBlueprintResources/StandardMacros.DoOnce` false
    (:`Completed`
      (`SceneComponent.SetHiddenInGame` OverlappedComponent true true)
      (`/Game/BP_BowlingBall.RemoveBallsEndLevelFour` (`self.Bowling Ball REF`) (`KismetStringLibrary.Conv_StringToInt` (`KismetTextLibrary.Conv_TextToString` (`TextRenderComponent.Text` (`self.Ball8_Text`)))) "X7"))))

(event `self.Ball9.OnComponentBeginOverlap`
  (params (OverlappedComponent :type "PrimitiveComponent Object Reference") (OtherActor :type "Actor Object Reference") (OtherComp :type "PrimitiveComponent Object Reference") (OtherBodyIndex :type Integer) (bFromSweep :type Boolean) (SweepResult :type "HitResult Structure (by ref)"))
  (`/Engine/EditorBlueprintResources/StandardMacros.DoOnce` false
    (:`Completed`
      (`SceneComponent.SetHiddenInGame` OverlappedComponent true true)
      (`/Game/BP_BowlingBall.RemoveBallsEndLevelFour` (`self.Bowling Ball REF`) (`KismetStringLibrary.Conv_StringToInt` (`KismetTextLibrary.Conv_TextToString` (`TextRenderComponent.Text` (`self.Ball9_Text`)))) "X7"))))

(event `self.Ball10.OnComponentBeginOverlap`
  (params (OverlappedComponent :type "PrimitiveComponent Object Reference") (OtherActor :type "Actor Object Reference") (OtherComp :type "PrimitiveComponent Object Reference") (OtherBodyIndex :type Integer) (bFromSweep :type Boolean) (SweepResult :type "HitResult Structure (by ref)"))
  (`/Engine/EditorBlueprintResources/StandardMacros.DoOnce` false
    (:`Completed`
      (`SceneComponent.SetHiddenInGame` OverlappedComponent true true)
      (`/Game/BP_BowlingBall.RemoveBallsEndLevelFour` (`self.Bowling Ball REF`) (`KismetStringLibrary.Conv_StringToInt` (`KismetTextLibrary.Conv_TextToString` (`TextRenderComponent.Text` (`self.Ball10_Text`)))) "X10"))))

(event `self.Ball11.OnComponentBeginOverlap`
  (params (OverlappedComponent :type "PrimitiveComponent Object Reference") (OtherActor :type "Actor Object Reference") (OtherComp :type "PrimitiveComponent Object Reference") (OtherBodyIndex :type Integer) (bFromSweep :type Boolean) (SweepResult :type "HitResult Structure (by ref)"))
  (`/Engine/EditorBlueprintResources/StandardMacros.DoOnce` false
    (:`Completed`
      (`SceneComponent.SetHiddenInGame` OverlappedComponent true true)
      (`/Game/BP_BowlingBall.RemoveBallsEndLevelFour` (`self.Bowling Ball REF`) (`KismetStringLibrary.Conv_StringToInt` (`KismetTextLibrary.Conv_TextToString` (`TextRenderComponent.Text` (`self.Ball11_Text`)))) "X10"))))

(event `self.Ball12.OnComponentBeginOverlap`
  (params (OverlappedComponent :type "PrimitiveComponent Object Reference") (OtherActor :type "Actor Object Reference") (OtherComp :type "PrimitiveComponent Object Reference") (OtherBodyIndex :type Integer) (bFromSweep :type Boolean) (SweepResult :type "HitResult Structure (by ref)"))
  (`/Engine/EditorBlueprintResources/StandardMacros.DoOnce` false
    (:`Completed`
      (`SceneComponent.SetHiddenInGame` OverlappedComponent true true)
      (`/Game/BP_BowlingBall.RemoveBallsEndLevelFour` (`self.Bowling Ball REF`) (`KismetStringLibrary.Conv_StringToInt` (`KismetTextLibrary.Conv_TextToString` (`TextRenderComponent.Text` (`self.Ball12_Text`)))) "X10"))))

(event `self.ReceiveBeginPlay`
  (`parent.ReceiveBeginPlay`)
  (`self.Set Number` (`self.Ball1_Text`))
  (`self.Set Number` (`self.Ball2_Text`))
  (`self.Set Number` (`self.Ball3_Text`))
  (`self.Set Number` (`self.Ball4_Text`))
  (`self.Set Number` (`self.Ball5_Text`))
  (`self.Set Number` (`self.Ball6_Text`))
  (`self.Set Number` (`self.Ball7_Text`))
  (`self.Set Number` (`self.Ball8_Text`))
  (`self.Set Number` (`self.Ball9_Text`))
  (`self.Set Number` (`self.Ball10_Text`))
  (`self.Set Number` (`self.Ball11_Text`))
  (`self.Set Number` (`self.Ball12_Text`))
  (bind _returnvalue (`GameplayStatics.GetActorOfClass` "/Game/BP_BowlingBall.BP_BowlingBall_C"))
  (set `self.Bowling Ball REF` _returnvalue))

(event `self.ReceiveTick`
  (params (DeltaSeconds :type "Float (single-precision)"))
  (`parent.ReceiveTick` DeltaSeconds))

(event `self.Impulse Collider.OnComponentBeginOverlap`
  (params (OverlappedComponent :type "PrimitiveComponent Object Reference") (OtherActor :type "Actor Object Reference") (OtherComp :type "PrimitiveComponent Object Reference") (OtherBodyIndex :type Integer) (bFromSweep :type Boolean) (SweepResult :type "HitResult Structure (by ref)"))
  (`PrimitiveComponent.SetSimulatePhysics` OtherComp true)
  (`PrimitiveComponent.SetCollisionEnabled` OtherComp "QueryAndPhysics")
  (`PrimitiveComponent.SetCollisionResponseToChannel` OtherComp "ECC_WorldStatic" "ECR_Block")
  (`PrimitiveComponent.AddImpulse` OtherComp (`KismetMathLibrary.MakeVector` (`KismetMathLibrary.RandomFloatInRange` 250.0 750.0) (`KismetMathLibrary.RandomFloatInRange` -200.0 200.0)) "None" true))

(fn `UserConstructionScript`
  (`parent.UserConstructionScript`))