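; End-of-level actor for level three that runs moving boxes which destroy BP_FollowBall actors on overlap.
; Tick slides a group of boxes along local Y by a fixed, frame-rate-dependent step.
; The Box trigger snaps any component entering it to a fixed relative location, which can recycle the moving boxes.
; Separate overlap events on individual boxes cast to BP_FollowBall and destroy it.
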(event `self.ReceiveTick`
  (params (DeltaSeconds :type "Float (single-precision)"))
  (`parent.ReceiveTick` DeltaSeconds)
  (`SceneComponent.K2_AddRelativeLocation` (`self.Box X15`) (0.0 5.0 0.0) false false)
  (`SceneComponent.K2_AddRelativeLocation` (`self.Box X2`) (0.0 5.0 0.0) false false)
  (`SceneComponent.K2_AddRelativeLocation` (`self.Box X3`) (0.0 5.0 0.0) false false)
  (`SceneComponent.K2_AddRelativeLocation` (`self.Box X7`) (0.0 5.0 0.0) false false)
  (`SceneComponent.K2_AddRelativeLocation` (`self.Box X5`) (0.0 5.0 0.0) false false)
  (`SceneComponent.K2_AddRelativeLocation` (`self.Box X10`) (0.0 5.0 0.0) false false))

(event `self.Box.OnComponentBeginOverlap`
  (params (OverlappedComponent :type "PrimitiveComponent Object Reference") (OtherActor :type "Actor Object Reference") (OtherComp :type "PrimitiveComponent Object Reference") (OtherBodyIndex :type Integer) (bFromSweep :type Boolean) (SweepResult :type "HitResult Structure (by ref)"))
  (`SceneComponent.K2_SetRelativeLocation` OtherComp (2150.0 -739.0 220.0) false false))

(event `self.Box X10.OnComponentBeginOverlap`
  (params (OverlappedComponent :type "PrimitiveComponent Object Reference") (OtherActor :type "Actor Object Reference") (OtherComp :type "PrimitiveComponent Object Reference") (OtherBodyIndex :type Integer) (bFromSweep :type Boolean) (SweepResult :type "HitResult Structure (by ref)"))
  (bind _asbp_follow_ball (cast `/Game/BP_FollowBall` OtherActor))
  (`self.K2_DestroyActor` _asbp_follow_ball))

(event `self.Box X5.OnComponentBeginOverlap`
  (params (OverlappedComponent :type "PrimitiveComponent Object Reference") (OtherActor :type "Actor Object Reference") (OtherComp :type "PrimitiveComponent Object Reference") (OtherBodyIndex :type Integer) (bFromSweep :type Boolean) (SweepResult :type "HitResult Structure (by ref)"))
  (bind _asbp_follow_ball (cast `/Game/BP_FollowBall` OtherActor))
  (`self.K2_DestroyActor` _asbp_follow_ball))

(event `self.Box X15.OnComponentBeginOverlap`
  (params (OverlappedComponent :type "PrimitiveComponent Object Reference") (OtherActor :type "Actor Object Reference") (OtherComp :type "PrimitiveComponent Object Reference") (OtherBodyIndex :type Integer) (bFromSweep :type Boolean) (SweepResult :type "HitResult Structure (by ref)"))
  (bind _asbp_follow_ball (cast `/Game/BP_FollowBall` OtherActor))
  (`self.K2_DestroyActor` _asbp_follow_ball))

(event `self.Box X2.OnComponentBeginOverlap`
  (params (OverlappedComponent :type "PrimitiveComponent Object Reference") (OtherActor :type "Actor Object Reference") (OtherComp :type "PrimitiveComponent Object Reference") (OtherBodyIndex :type Integer) (bFromSweep :type Boolean) (SweepResult :type "HitResult Structure (by ref)"))
  (bind _asbp_follow_ball (cast `/Game/BP_FollowBall` OtherActor))
  (`self.K2_DestroyActor` _asbp_follow_ball))

(event `self.Box X3.OnComponentBeginOverlap`
  (params (OverlappedComponent :type "PrimitiveComponent Object Reference") (OtherActor :type "Actor Object Reference") (OtherComp :type "PrimitiveComponent Object Reference") (OtherBodyIndex :type Integer) (bFromSweep :type Boolean) (SweepResult :type "HitResult Structure (by ref)"))
  (bind _asbp_follow_ball (cast `/Game/BP_FollowBall` OtherActor))
  (`self.K2_DestroyActor` _asbp_follow_ball))

(event `self.Box X7.OnComponentBeginOverlap`
  (params (OverlappedComponent :type "PrimitiveComponent Object Reference") (OtherActor :type "Actor Object Reference") (OtherComp :type "PrimitiveComponent Object Reference") (OtherBodyIndex :type Integer) (bFromSweep :type Boolean) (SweepResult :type "HitResult Structure (by ref)"))
  (bind _asbp_follow_ball (cast `/Game/BP_FollowBall` OtherActor))
  (`self.K2_DestroyActor` _asbp_follow_ball))

(fn `UserConstructionScript`
  (`parent.UserConstructionScript`))