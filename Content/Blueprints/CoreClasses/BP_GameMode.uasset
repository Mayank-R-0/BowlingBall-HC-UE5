(event `self.ReceiveBeginPlay`
  (bind _returnvalue (`|CreateWidget` "/Game/UI/MainMenu.MainMenu_C"))
  (set `self.Main UI ` _returnvalue)
  (`self.Load Rewarded Ad`)
  (`|ExecutionSequence`
    (:`then_1`
      (bind _returnvalue_2 (`GameplayStatics.LoadGameFromSlot` (`self.Slot Name`) (`self.User Index`)))
      (bind _asbp_save_game (cast `/Game/Blueprints/CoreClasses/BP_SaveGame` _returnvalue_2)
        (:`then`
          (set `self.SaveGame` _asbp_save_game))
        (:`CastFailed`
          (bind _returnvalue_3 (`GameplayStatics.CreateSaveGameObject` "/Game/Blueprints/CoreClasses/BP_SaveGame.BP_SaveGame_C"))
          (bind _output_get (set `self.SaveGame` _returnvalue_3))
          (set `/Game/Blueprints/CoreClasses/BP_SaveGame.TotalGems` 0 _output_get)
          (set `/Game/Blueprints/CoreClasses/BP_SaveGame.CurrentLevel` 1 (`self.SaveGame`))
          (`self.SaveTheGame`)))
      (bind _asbp_game_instance (cast `/Game/Blueprints/CoreClasses/BP_GameInstance` (`GameplayStatics.GetGameInstance`)))
      (set `/Game/Blueprints/CoreClasses/BP_GameInstance.TotalGems` (`/Game/Blueprints/CoreClasses/BP_SaveGame.TotalGems` (`self.SaveGame`)) _asbp_game_instance))))

(event `SaveTheGame`
  (`GameplayStatics.SaveGameToSlot` (`self.SaveGame`) (`self.Slot Name`) (`self.User Index`)))

(event `Load Rewarded Ad`
  (`AdMobBPLibrary.LoadRewardedVideo` 0 (delegate `Ad Loaded`) (delegate `Ad Failed`)))

(event `Ad Loaded`)

(event `Play Rewarded AD`
  (params (`Reward Type` :type "/Game/Blueprints/Enumerations/RewardType Enum" :default "NewEnumerator0") (Index :type Integer))
  (bind _asbp_game_instance (cast `/Game/Blueprints/CoreClasses/BP_GameInstance` (`GameplayStatics.GetGameInstance`)))
  (set `/Game/Blueprints/CoreClasses/BP_GameInstance.Reward Type` `Reward Type` _asbp_game_instance)
  (set `/Game/Blueprints/CoreClasses/BP_GameInstance.Free Ad Index` Index _asbp_game_instance)
  (`AdMobBPLibrary.PlayRewardedVideo` (delegate `Ad Opened`) (delegate `Ad Closed`) (delegate `Reward Earned`) (delegate `Failed`)))

(event `Ad Failed`
  (`KismetSystemLibrary.PrintString` "Ad Loading Failed")
  (bind _returnvalue (`GameplayStatics.GetCurrentLevelName` true))
  (`GameplayStatics.OpenLevel` (`KismetStringLibrary.Conv_StringToName` _returnvalue)))

(event `Ad Opened`
  (`KismetSystemLibrary.PrintString` "Ad Opened"))

(event `Ad Closed`
  (`KismetSystemLibrary.PrintString` "Ad Closed"))

(event `Failed`
  (`KismetSystemLibrary.PrintString` "Ad Failed"))

(event `Reward Earned`
  (params (reward :type "AdMobRewardItem Structure"))
  (bind _asbp_game_instance (cast `/Game/Blueprints/CoreClasses/BP_GameInstance` (`GameplayStatics.GetGameInstance`)))
  (bind _reward_type (`/Game/Blueprints/CoreClasses/BP_GameInstance.Reward Type` _asbp_game_instance))
  (`KismetSystemLibrary.PrintString` (`|GetEnumeratorNameAsString` _reward_type))
  (switch `/Game/Blueprints/Enumerations/RewardType` _reward_type
    (:`NewEnumerator0`
      (`KismetSystemLibrary.PrintString` "Map Level Up Reward Earned")
      (`KismetSystemLibrary.Delay` 1.0)
      (bind _asbp_game_instance_2 (cast `/Game/Blueprints/CoreClasses/BP_GameInstance` (`GameplayStatics.GetGameInstance`)))
      (bind _returnvalue (+ (`/Game/Blueprints/CoreClasses/BP_GameInstance.CurrentLevel` _asbp_game_instance_2) 1))
      (bind _output_get (set `/Game/Blueprints/CoreClasses/BP_GameInstance.CurrentLevel` (`KismetMathLibrary.SelectInt` _returnvalue 1 (<= _returnvalue 100)) _asbp_game_instance_2))
      (`GameplayStatics.OpenLevel` (`KismetStringLibrary.Conv_StringToName` (`KismetStringLibrary.Concat_StrStr` "Map" (`KismetStringLibrary.Conv_IntToString` _output_get))))
      (`self.Load Rewarded Ad`))
    (:`NewEnumerator1`
      (`KismetSystemLibrary.Delay` 0.1)
      (`self.Reward Earn` (`/Game/Blueprints/CoreClasses/BP_GameInstance.Free Ad Index` _asbp_game_instance))
      (`self.Load Rewarded Ad`))))

(fn `UserConstructionScript`)