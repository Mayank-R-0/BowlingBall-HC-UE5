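; BP_FollowSpline is an actor that moves two reference points along its spline at MovementSpeed until PauseSpline is set.
; Tick accumulates distance and applies the spline's local transform to CameraReferencePoint and to ReferencePoint, which is also shifted along its right vector by Offset.
; BeginPlay unhides the TextRender in game.
; Construction script logic for tiling instanced meshes along the spline is disconnected and never runs.
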(event `self.ReceiveBeginPlay`
  (`SceneComponent.SetHiddenInGame` (`self.TextRender`) false false))

(event `self.ReceiveTick`
  (params (DeltaSeconds :type "Float (single-precision)"))
  (bind _referencepoint (`self.ReferencePoint`))
  (bind _camerareferencepoint (`self.CameraReferencePoint`))
  (if (not (`self.Pause Spline`))
    (bind _output_get (set `self.DistanceCoveredAlongSpline'` (+ (* DeltaSeconds (`self.MovementSpeed`)) (`self.DistanceCoveredAlongSpline'`))))
    (bind (_returnvalue_location _returnvalue_rotation) (`KismetMathLibrary.BreakTransform` (`SplineComponent.GetTransformAtDistanceAlongSpline` (`self.Spline`) _output_get "Local" false)))
    (`SceneComponent.K2_SetRelativeTransform` _referencepoint (`KismetMathLibrary.MakeTransform` (+ _returnvalue_location (* (`KismetMathLibrary.Normal` (`SceneComponent.GetRightVector` (`self.ReferencePoint`))) (`self.Offset`))) _returnvalue_rotation (`SceneComponent.RelativeScale3D` _referencepoint)) false false)
    (`SceneComponent.K2_SetRelativeTransform` _camerareferencepoint (`KismetMathLibrary.MakeTransform` _returnvalue_location _returnvalue_rotation (`SceneComponent.RelativeScale3D` _camerareferencepoint)) false false)))

(fn `Get LocationAtIndex`
  (params (A :type Integer))
  (returns (ReturnValue :type "Vector Structure"))
  (return (`SplineComponent.GetLocationAtDistanceAlongSpline` (`self.Spline`) (* A (`self.Spacing`)) "Local")))

(fn `UserConstructionScript`
  (locals (`Number of instance` :type Integer :default 0)))