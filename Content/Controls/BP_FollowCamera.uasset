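; BP_FollowCamera is a camera actor with a spring arm that animates a transition when LerpCamera is called.
; The event captures the current transform and targets a location shifted along world X by the given Offset.
; The Lerping timeline then blends the actor to that location and toward zero rotation, while easing the spring arm pitch from angled down to level.
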(event `LerpCamera`
  (params (Offset :type "Float (double-precision)"))
  (bind _returnvalue (`self.K2_GetActorLocation`))
  (set `self.StartRotation` (`self.K2_GetActorRotation`))
  (set `self.StartLocation` _returnvalue)
  (set `self.EndLocation` (`KismetMathLibrary.MakeVector` (+ (.x _returnvalue) Offset) (.y _returnvalue) (.z _returnvalue)))
  (bind (_direction _alpha) (`Timeline|Lerping`)
    (:`Update`
      (`self.K2_SetActorLocation` (`KismetMathLibrary.VLerp` (`self.StartLocation`) (`self.EndLocation`) _alpha))
      (`self.K2_SetActorRotation` (`KismetMathLibrary.RLerp` (`self.StartRotation`) (struct) _alpha))
      (`SceneComponent.K2_SetRelativeRotation` (`self.SpringArm`) (`KismetMathLibrary.MakeRotator` 0.0 (`KismetMathLibrary.Lerp` -45.0 0.0 _alpha)) false false))))

(fn `UserConstructionScript`)