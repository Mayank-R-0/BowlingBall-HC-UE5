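; BP_FollowBall is a follower ball that trails a head actor in one of five columns and destroys itself on hitting typed obstacles.
; FollowTarget interpolates it toward an offset along the head's forward and right vectors, turning to face its movement.
; If the head is invalid, it retargets MainBall and derives the sideways offset from ColumnNumber.
; Sphere overlaps check TypeInterface; the call to MainBall's ResetReferences is disconnected.
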(event `FollowTarget`
  (bind _returnvalue (`GameplayStatics.GetWorldDeltaSeconds`))
  (bind _followingspeed (`self.FollowingSpeed`))
  (bind _returnvalue_2 (`KismetMathLibrary.VInterpTo` (`self.K2_GetActorLocation`) (+ (`self.K2_GetActorLocation` (`self.FollowHead`)) (+ (* (`KismetMathLibrary.Normal` (`self.GetActorForwardVector` (`self.FollowHead`))) (`self.Offset`)) (* (`KismetMathLibrary.Normal` (`self.GetActorRightVector` (`self.FollowHead`))) (`self.Yoffset`)))) _returnvalue _followingspeed))
  (`/Engine/EditorBlueprintResources/StandardMacros.IsValid` (`self.FollowHead`)
    (:`Is Valid`
      (`self.K2_SetActorLocationAndRotation` _returnvalue_2 (`KismetMathLibrary.RInterpTo` (`self.K2_GetActorRotation`) (`KismetMathLibrary.FindLookAtRotation` (`self.K2_GetActorLocation`) _returnvalue_2) _returnvalue _followingspeed)))
    (:`Is Not Valid`
      (`/Engine/EditorBlueprintResources/StandardMacros.DoOnce` false :!label _label
        (:`Completed`
          (set `self.FollowHead` (`self.MainBall`))
          (switch `int` (`self.ColumnNumber`)
            (:`0`
              (set `self.Yoffset` -100.0)
              (goto _label :!via `Reset`))
            (:`1`
              (set `self.Yoffset` -50.0)
              (goto _label :!via `Reset`))
            (:`2`
              (set `self.Yoffset` 0.0)
              (goto _label :!via `Reset`))
            (:`3`
              (set `self.Yoffset` 50.0)
              (goto _label :!via `Reset`))
            (:`4`
              (set `self.Yoffset` 100.0)
              (goto _label :!via `Reset`))))))))

(event `self.Sphere.OnComponentBeginOverlap`
  (params (OverlappedComponent :type "PrimitiveComponent Object Reference") (OtherActor :type "Actor Object Reference") (OtherComp :type "PrimitiveComponent Object Reference") (OtherBodyIndex :type Integer) (bFromSweep :type Boolean) (SweepResult :type "HitResult Structure (by ref)"))
  (bind _astype_interface (cast `/Game/TypeInterface` OtherActor))
  (bind _type (`/Game/TypeInterface.GetObstType` _astype_interface))
  (switch `/Game/ObstacleType` _type
    (:`NewEnumerator0`
      _)
    (:`NewEnumerator1`
      _)
    (:`NewEnumerator2`
      _))
  (`self.K2_DestroyActor`))

(fn `UserConstructionScript`)